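; BP_TrapSpike is a spike trap Blueprint that supplies the visual effect for trap damage.
; Its PlayDamageVFX event spawns a scaled-down Niagara lightning aura attached above SceneRoot, set to auto-destroy, and activates it.
; An unconnected spawn-at-location variant remains in the graph, noted as failing to destroy.
; The file holds no other active gameplay logic.
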(event `self.PlayDamageVFX`
  (params (EffectLocation :type "Vector Structure"))
  (bind _returnvalue (`NiagaraFunctionLibrary.SpawnSystemAttached` "/Game/VFX/FreeSpells/VFX_Niagara/NS_Free_Spells_Aura_Lightning.NS_Free_Spells_Aura_Lightning" (`self.SceneRoot`) "None" (0.0 0.0 70.0) (struct) "KeepRelativeOffset" true))
  (`SceneComponent.SetRelativeScale3D` _returnvalue (0.7 0.7 0.7))
  (`ActorComponent.Activate` _returnvalue true))

(fn `UserConstructionScript`
  (`parent.UserConstructionScript`))