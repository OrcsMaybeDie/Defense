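; Pistol weapon Blueprint that supplies the cosmetic firing feedback for normal and charged shots.
; OnWeaponAction branches on action type: Fire restarts the Niagara effect and plays a shotgun fire sound at the weapon mesh's muzzle socket.
; Executed Charged Fire reuses that feedback at stage 1 and switches to Charge2VFX with a penetrating-shot sound at stage 2.
; Stage 3 has no connected behavior, only an orphaned debug print.
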(event `self.OnWeaponAction`
  (params (ActionType :type "EWeaponActionType Enum" :default "Fire") (Phase :type "EWeaponActionPhase Enum" :default "Started") (ChargeStage :type "EWeaponChargeStage Enum" :default "None") (ChargeRatio :type "Float (single-precision)"))
  (bind _charge2vfx (`self.Charge2VFX`))
  (switch `EWeaponActionType` ActionType
    (:`Fire`
      (`ActorComponent.Activate` (`self.Niagara`) true :!label _label)
      (`GameplayStatics.PlaySoundAtLocation` "/Game/Audio/Sounds/Weapons/Shotgun/MSS_Weapons_Shotgun_Fire.MSS_Weapons_Shotgun_Fire" (`SceneComponent.GetSocketLocation` (`self.WeaponMesh`) "Muzzle") (struct) 1.0 1.0 0.0 null null null null))
    (:`ChargedFire`
      (switch `EWeaponActionPhase` Phase
        (:`Executed`
          (switch `EWeaponChargeStage` ChargeStage
            (:`Stage1`
              (goto _label))
            (:`Stage2`
              (`ActorComponent.Activate` _charge2vfx false)
              (`GameplayStatics.PlaySoundAtLocation` "/Game/_Defense/VFX/Weapons/Pistol/Stage2_PenetratingShot/SFX/EVFX04_16_PenetratingShot.EVFX04_16_PenetratingShot" (`SceneComponent.GetSocketLocation` _charge2vfx "Muzzle") (struct) 1.0 1.0 0.0 null null null null))))))))

(fn `UserConstructionScript`)