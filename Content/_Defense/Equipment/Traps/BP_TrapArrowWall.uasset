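; Arrow wall trap for the defense equipment that supplies the cosmetic side of a wall shot.
; PlayWallShotVFX spawns three BP_ArrowWallVisual actors in a row along the trap's right vector, each rotated toward the shot's end point.
; Each visual receives the original, un-offset start and end locations, and spawning is skipped on dedicated servers.
; This graph holds no trigger, targeting or damage logic.
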(event `self.PlayWallShotVFX`
  (params (StartLocation :type "Vector Structure") (EndLocation :type "Vector Structure"))
  (if (not (`KismetSystemLibrary.IsDedicatedServer`))
    (for _index (range 3)
      (bind _returnvalue (+ StartLocation (* (`self.GetActorRightVector`) (- (* _index 80) 80))))
      (`|SpawnActorFromClass` "/Game/_Defense/Equipment/Traps/BP_ArrowWallVisual.BP_ArrowWallVisual_C" (`KismetMathLibrary.MakeTransform` _returnvalue (`KismetMathLibrary.FindLookAtRotation` _returnvalue EndLocation)) "Undefined" "MultiplyWithRoot" null StartLocation EndLocation null))))

(fn `UserConstructionScript`
  (`parent.UserConstructionScript`))